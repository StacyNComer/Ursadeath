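; BP_UrsadeathGameInstance is the Ursadeath game instance, which applies the player's saved audio volumes.
; The LoadAudioSettings event reads master, enemy SFX, player SFX and music volumes from the Ursadeath user settings.
; Each volume becomes a sound class override on its own sound mix, which is then pushed as a modifier.
; An empty ConvenientTestFunc is also present.
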(event `self.LoadAudioSettings`
  (bind _returnvalue (`UrsadeathUserSettings.GetUrsadeathUserSettings`))
  (`|ExecutionSequence`
    (:`then_0`
      (`GameplayStatics.SetSoundMixClassOverride` "/Game/Ursadeath/Core/Blueprints/Audio/SoundMixes/SCM_Master.SCM_Master" "/Game/Ursadeath/Core/Blueprints/Audio/SoundClasses/SC_Master.SC_Master" (`UrsadeathUserSettings.GetMasterVolume` _returnvalue))
      (`GameplayStatics.PushSoundMixModifier` "/Game/Ursadeath/Core/Blueprints/Audio/SoundMixes/SCM_Master.SCM_Master"))
    (:`then_1`
      (`GameplayStatics.SetSoundMixClassOverride` "/Game/Ursadeath/Core/Blueprints/Audio/SoundMixes/SCM_EnemySFX.SCM_EnemySFX" "/Game/Ursadeath/Core/Blueprints/Audio/SoundClasses/SC_EnemySFX.SC_EnemySFX" (`UrsadeathUserSettings.GetEnemySFXVolume` _returnvalue))
      (`GameplayStatics.PushSoundMixModifier` "/Game/Ursadeath/Core/Blueprints/Audio/SoundMixes/SCM_EnemySFX.SCM_EnemySFX"))
    (:`then_2`
      (`GameplayStatics.SetSoundMixClassOverride` "/Game/Ursadeath/Core/Blueprints/Audio/SoundMixes/SCM_PlayerSFX.SCM_PlayerSFX" "/Game/Ursadeath/Core/Blueprints/Audio/SoundClasses/SC_PlayerSFX.SC_PlayerSFX" (`UrsadeathUserSettings.GetPlayerSFXVolume` _returnvalue))
      (`GameplayStatics.PushSoundMixModifier` "/Game/Ursadeath/Core/Blueprints/Audio/SoundMixes/SCM_PlayerSFX.SCM_PlayerSFX"))
    (:`then_3`
      (`GameplayStatics.SetSoundMixClassOverride` "/Game/Ursadeath/Core/Blueprints/Audio/SoundMixes/SCM_Music.SCM_Music" "/Game/Ursadeath/Core/Blueprints/Audio/SoundClasses/SC_Music.SC_Music" (`UrsadeathUserSettings.GetMusicVolume` _returnvalue))
      (`GameplayStatics.PushSoundMixModifier` "/Game/Ursadeath/Core/Blueprints/Audio/SoundMixes/SCM_Music.SCM_Music"))))

(fn `Convenient Test Func`)