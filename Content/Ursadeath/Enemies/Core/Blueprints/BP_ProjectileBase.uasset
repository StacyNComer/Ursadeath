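; Base enemy projectile for Ursadeath that damages the player on contact.
; When its sphere overlaps the player, it calls DamagePlayer with its Damage value and destroys itself.
; It passes through UDEnemy actors and projectiles of exactly this class, and destroys itself on any other overlap.
; The projectile check is an exact class match, so child projectile classes are not exempt.
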(event `self.ReceiveActorBeginOverlap`
  (params (OtherActor :type "Actor Object Reference")))

(event `self.Sphere1.OnComponentBeginOverlap`
  (params (OverlappedComponent :type "PrimitiveComponent Object Reference") (OtherActor :type "Actor Object Reference") (OtherComp :type "PrimitiveComponent Object Reference") (OtherBodyIndex :type Integer) (bFromSweep :type Boolean) (SweepResult :type "HitResult Structure (by ref)"))
  (bind _returnvalue (`GameplayStatics.GetObjectClass` OtherActor))
  (bind _asbp_ursadeath_player (cast `/Game/Ursadeath/PlayerCharacter/Blueprints/BP_UrsadeathPlayer` OtherActor)
    (:`then`
      (`UDPlayerCharacter.DamagePlayer` _asbp_ursadeath_player (`self.Damage`))
      (`self.K2_DestroyActor` :!label _label))
    (:`CastFailed`
      (if (not (or (`KismetMathLibrary.ClassIsChildOf` _returnvalue "/Script/Ursadeath.UDEnemy") (== _returnvalue "BP_ProjectileBase_C")))
        (goto _label)))))

(fn `UserConstructionScript`)