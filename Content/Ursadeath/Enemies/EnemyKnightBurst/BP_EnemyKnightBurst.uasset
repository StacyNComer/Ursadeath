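; Burst-firing Knight enemy for Ursadeath that takes 50% longer stuns from attacks.
; Sight perception feeds the blackboard's player-visibility flag, and firing is blocked briefly after spawning.
; Shoot halts movement, plays a warning effect and charge sound, then uses a restarting timeline to space three projectile shots.
; Interruption zeroes the remaining bursts and stops the timeline.
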(event `self.ReceiveBeginPlay`
  (add `self.OnAttackRecieved` (delegate `Stun Weakness`)))

(event `Stun Weakness` :!signature `self.OnAttackRecieved`
  (params (DamageData :type "UDPlayerAttackData Object Reference"))
  (bind (_attackstats_attacktype _attackstats_damage _attackstats_stuntime) (break `PlayerAttackStats` (`UDPlayerAttackData.AttackStats` DamageData)))
  (bind (_attackstats_attacktype_2 _attackstats_damage_2 _attackstats_stuntime_2) (break `PlayerAttackStats` (`UDPlayerAttackData.AttackStats` DamageData)))
  (if (> _attackstats_stuntime_2 0.0)
    (set `UDPlayerAttackData.AttackStats` (make `PlayerAttackStats` "PRIMARY_FIRE" _attackstats_damage (* _attackstats_stuntime 1.5)) DamageData)))

(event `self.OnSpawnSequenceEnd`
  (`BlackboardComponent.SetValueAsBool` (`AIBlueprintHelperLibrary.GetBlackboard` null) "CanSeePlayer?" (`KismetArrayLibrary.Array_Contains` (`AIPerceptionComponent.GetCurrentlyPerceivedActors` (`self.AIPerception`) "/Script/AIModule.AISense_Sight") (`UDPlayerCharacter.GetCharacterInPlay`)))
  (`BlackboardComponent.SetValueAsBool` (`AIBlueprintHelperLibrary.GetBlackboard` null) "NoFire" true)
  (`KismetSystemLibrary.Delay` (`self.SpawnFireDelay`))
  (`BlackboardComponent.SetValueAsBool` (`AIBlueprintHelperLibrary.GetBlackboard` null) "NoFire" false))

(event `self.ReceiveTick`
  (params (DeltaSeconds :type "Float (single-precision)")))

(event `Shoot`
  (`MovementComponent.StopMovementImmediately` (`self.FloatingPawnMovement`))
  (`NiagaraFunctionLibrary.SpawnSystemAttached` "/Game/Ursadeath/Enemies/Core/ParticleFX/NS_EnemyAttackWarning.NS_EnemyAttackWarning" (`self.GunFXSpawn`) "Muzzle_Front" (0.0 0.0 0.0) (struct) "KeepRelativeOffset" true)
  (`GameplayStatics.PlaySoundAtLocation` "/Game/Ursadeath/Enemies/EnemyKnightBurst/Burst_Charge.Burst_Charge" (`self.K2_GetActorLocation`) (struct) 1.0 1.0 0.0 null null null null)
  (`BlackboardComponent.SetValueAsBool` (`AIBlueprintHelperLibrary.GetBlackboard` null) "IsFiring?" true)
  (set `self.Bursts Remaining` 3)
  (`TimelineComponent.PlayFromStart` (`self.TL_BurstDelay`)))

(event `self.AIPerception.OnTargetPerceptionUpdated`
  (params (Actor :type "Actor Object Reference") (Stimulus :type "AIStimulus Structure"))
  (bind _returnvalue (`AIBlueprintHelperLibrary.GetBlackboard` null))
  (cast `/Game/Ursadeath/PlayerCharacter/Blueprints/BP_UrsadeathPlayer` Actor)
  (`/Engine/EditorBlueprintResources/StandardMacros.IsValid` _returnvalue
    (:`Is Valid`
      (`BlackboardComponent.SetValueAsBool` _returnvalue "CanSeePlayer?" Stimulus_bSuccessfullySensed))))

(event `self.OnInterrupted`
  (params (WasAlreadyStunned :type Boolean))
  ;[1 1 1] Stops the enemy's burst fire
  (set `self.Bursts Remaining` 0)
  (`TimelineComponent.Stop` (`self.TL_BurstDelay`)))

(fn `UserConstructionScript`)