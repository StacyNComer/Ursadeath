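; Dashing enemy that charges across the arena to damage the player, coordinated with its AI through blackboard keys.
; Dash sphere-traces forward for a destination, pauses to charge, bursts at high speed, then toggles DashReady for a random cooldown.
; Dash collision and a gated sphere overlap deal damage; NoFire is held briefly after spawning.
; Slow-on-damage and rocket-weakness logic exists, but its binding here is unwired.
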(event `self.OnSpawnSequenceEnd`
  (set `self.Base Speed` (`MovementComponent.GetMaxSpeed` (`self.FloatingPawnMovement`))) ; Record the base speed of the enemy
  (`BlackboardComponent.SetValueAsBool` (`AIBlueprintHelperLibrary.GetBlackboard` null) "DashReady" true)
  (`BlackboardComponent.SetValueAsBool` (`AIBlueprintHelperLibrary.GetBlackboard` null) "NoFire" true)
  (`KismetSystemLibrary.Delay` (`KismetMathLibrary.RandomFloatInRange` (`self.MinSpawnDashDelay`) (`self.MaxSpawnDashDelay`)))
  (`BlackboardComponent.SetValueAsBool` (`AIBlueprintHelperLibrary.GetBlackboard` null) "NoFire" false))

(event `self.ReceiveBeginPlay`
  (`parent.ReceiveBeginPlay`))

(event `Damage Weaknesses` :!signature `self.OnAttackRecieved`
  (params (DamageData :type "UDPlayerAttackData Object Reference"))
  (bind (_attackstats_attacktype _attackstats_damage _attackstats_stuntime) (break `PlayerAttackStats` (`UDPlayerAttackData.AttackStats` DamageData)))
  (bind (_attackstats_attacktype_2 _attackstats_damage_2 _attackstats_stuntime_2) (break `PlayerAttackStats` (`UDPlayerAttackData.AttackStats` DamageData)))
  (`|ExecutionSequence`
    (:`then_0`
      (if (or (> _attackstats_damage_2 0) (> _attackstats_stuntime_2 0.0))
        (`self.ApplySlow` (`self.Slow Time`))))
    (:`then_1`
      ;[1 1 1] Rocket Weakness
      (if (`|EnumEquality` _attackstats_attacktype "ROCKET")
        (`UDPlayerAttackData.SetDamage` DamageData (`KismetMathLibrary.FTrunc` (* _attackstats_damage 1.5)))
        (`UDPlayerAttackData.SetStunTime` DamageData (+ _attackstats_stuntime (`self.Rocket Stun Time`)))))))

(event `self.ReceiveTick`
  (params (DeltaSeconds :type "Float (single-precision)"))
  (`parent.ReceiveTick` DeltaSeconds))

(event `self.Sphere2.OnComponentBeginOverlap`
  (params (OverlappedComponent :type "PrimitiveComponent Object Reference") (OtherActor :type "Actor Object Reference") (OtherComp :type "PrimitiveComponent Object Reference") (OtherBodyIndex :type Integer) (bFromSweep :type Boolean) (SweepResult :type "HitResult Structure (by ref)"))
  (if (and (`self.CanDamageCircleDash`) (!= (`self.IsStunned`) true))
    (bind _asbp_ursadeath_player (cast `/Game/Ursadeath/PlayerCharacter/Blueprints/BP_UrsadeathPlayer` OtherActor))
    (`UDPlayerCharacter.DamagePlayer` _asbp_ursadeath_player (`self.Damage_Punch`))))

(event `self.Dash_Collision.OnComponentBeginOverlap`
  (params (OverlappedComponent :type "PrimitiveComponent Object Reference") (OtherActor :type "Actor Object Reference") (OtherComp :type "PrimitiveComponent Object Reference") (OtherBodyIndex :type Integer) (bFromSweep :type Boolean) (SweepResult :type "HitResult Structure (by ref)"))
  (bind _asbp_ursadeath_player (cast `/Game/Ursadeath/PlayerCharacter/Blueprints/BP_UrsadeathPlayer` OtherActor))
  (`UDPlayerCharacter.DamagePlayer` _asbp_ursadeath_player (`self.Damage_Dash`))
  (`PrimitiveComponent.SetCollisionEnabled` (`self.Dash_Collision`) "NoCollision"))

(event `Dash Location`
  (bind _arrow (`self.Arrow`))
  (bind _returnvalue (`SceneComponent.K2_GetComponentLocation` _arrow))
  (bind (_returnvalue_x _returnvalue_y _returnvalue_z) (`KismetMathLibrary.BreakVector` (+ _returnvalue (* (`SceneComponent.GetForwardVector` _arrow) (`UDCoreLibrary.GetArenaDiameter`)))))
  (bind _outhit (`KismetSystemLibrary.SphereTraceSingleForObjects` _returnvalue (`KismetMathLibrary.MakeVector` _returnvalue_x _returnvalue_y _returnvalue_z) 20.0 (`|MakeArray` "ObjectTypeQuery1" "ObjectTypeQuery2" "ObjectTypeQuery12" :!type "EObjectTypeQuery Enum")))
  (`|AIMoveTo` self (`.ImpactPoint` (`GameplayStatics.BreakHitResult` _outhit)) null 10.0))

(event `Dash`
  (bind _returnvalue (`self.K2_GetActorLocation`))
  (`PrimitiveComponent.SetCollisionEnabled` (`self.Dash_Collision`) "QueryOnly")
  (`self.Dash Location`)
  (if (not (`self.IsDashing?`))
    (set `self.IsDashing?` true)
    (set `FloatingPawnMovement.MaxSpeed` 0.0 (`self.FloatingPawnMovement`))
    (`GameplayStatics.PlaySoundAtLocation` "/Game/Ursadeath/Enemies/EnemyKnightDash/Charging_Sound.Charging_Sound" _returnvalue (struct) 1.0 1.0 0.0 null null null null)
    (`KismetSystemLibrary.Delay` (`self.Dash Delay`))
    (set `FloatingPawnMovement.MaxSpeed` (`self.Dashing Speed`) (`self.FloatingPawnMovement`))
    (`GameplayStatics.PlaySoundAtLocation` "/Game/Ursadeath/Enemies/EnemyKnightDash/Dash_Sound.Dash_Sound" _returnvalue (struct) 1.0 1.0 0.0 null null null null)
    (`KismetSystemLibrary.Delay` 1.0)
    (set `FloatingPawnMovement.MaxSpeed` (`self.Base Speed`) (`self.FloatingPawnMovement`))
    (set `self.IsDashing?` false)
    (`PrimitiveComponent.SetCollisionEnabled` (`self.Dash_Collision`) "NoCollision")
    (`BlackboardComponent.SetValueAsBool` (`AIBlueprintHelperLibrary.GetBlackboard` null) "DashReady" false)
    (`KismetSystemLibrary.Delay` (`KismetMathLibrary.RandomFloatInRange` 3.0 5.0))
    (`BlackboardComponent.SetValueAsBool` (`AIBlueprintHelperLibrary.GetBlackboard` null) "DashReady" true)))

(fn `UserConstructionScript`
  (`parent.UserConstructionScript`))