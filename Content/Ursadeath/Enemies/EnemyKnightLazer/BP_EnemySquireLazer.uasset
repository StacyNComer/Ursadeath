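; Laser-firing squire enemy that takes extra damage from melee attacks and briefly holds fire after spawning.
; Shoot shows a thin warning beam during a timeline charge, then fires the large beam for three seconds with controller yaw locked.
; Tick sphere-traces to set beam length and damage the player on a cooldown.
; Sight perception and firing state feed the AI blackboard, and a stun interrupt shuts the laser down.
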(event `self.ReceiveBeginPlay`
  ;[1 1 1] Stops effect/audio on spawm
  (add `self.OnAttackRecieved` (delegate `Melee Weakness`))
  (`AudioComponent.Stop` (`self.AudioFiringLaser`))
  (`AudioComponent.Stop` (`self.AudioChargingLaser`)))

(event `Melee Weakness` :!signature `self.OnAttackRecieved`
  (params (DamageData :type "UDPlayerAttackData Object Reference"))
  (bind (_attackstats_attacktype _attackstats_damage) (break `PlayerAttackStats` (`UDPlayerAttackData.AttackStats` DamageData)))
  ;[1 1 1] Weak to Melee Attacks
  (if (`|EnumEquality` _attackstats_attacktype "MELEE")
    (`UDPlayerAttackData.SetDamage` DamageData (* _attackstats_damage 1.5))))

(event `self.OnSpawnSequenceEnd`
  ;[1 1 1] Making sure the enemy can see the player on spawn and not fire for a short duration
  (`BlackboardComponent.SetValueAsBool` (`AIBlueprintHelperLibrary.GetBlackboard` null) "CanSeePlayer?" false)
  (`BlackboardComponent.SetValueAsBool` (`AIBlueprintHelperLibrary.GetBlackboard` null) "NoFire" true)
  (`KismetSystemLibrary.Delay` (`self.SpawnFireDelay`))
  (`BlackboardComponent.SetValueAsBool` (`AIBlueprintHelperLibrary.GetBlackboard` null) "NoFire" false)
  (`BlackboardComponent.SetValueAsBool` (`AIBlueprintHelperLibrary.GetBlackboard` null) "CanSeePlayer?" (`KismetArrayLibrary.Array_Contains` (`AIPerceptionComponent.GetCurrentlyPerceivedActors` (`self.AIPerception`) "/Script/AIModule.AISense_Sight") (`UDPlayerCharacter.GetCharacterInPlay`))))

(event `self.ReceiveTick`
  (params (DeltaSeconds :type "Float (single-precision)"))
  (bind _weapon_attack_spawn (`self.Weapon Attack Spawn`))
  (bind _returnvalue (`SceneComponent.K2_GetComponentLocation` _weapon_attack_spawn))
  ;[1 1 1] Logic for figuring out where to fire
  (`|ExecutionSequence`
    (:`then_0`
      ;[1 1 1] Decrement laser damage cooldown
      (if (> (`self.Cooldown_Tracker`) 0.0)
        (set `self.Cooldown_Tracker` (- (`self.Cooldown_Tracker`) DeltaSeconds))))
    (:`then_1`
      (if (`self.LazerIsFiring?`)
        (bind _outhit (`KismetSystemLibrary.SphereTraceSingleForObjects` _returnvalue (+ _returnvalue (* (`SceneComponent.GetForwardVector` _weapon_attack_spawn) (`UDCoreLibrary.GetArenaDiameter`))) 20.0 (`|MakeArray` "ObjectTypeQuery1" "ObjectTypeQuery8" "ObjectTypeQuery2" "ObjectTypeQuery12" :!type "EObjectTypeQuery Enum")))
        (bind (_bblockinghit _binitialoverlap _time _distance _location _impactpoint _normal _impactnormal _physmat _hitactor) (`GameplayStatics.BreakHitResult` _outhit))
        (if _bblockinghit
          (`NiagaraComponent.SetVariableVec3` (`self.Laser FX`) "User.Beam_End" (`KismetMathLibrary.MakeVector` _distance))
          (`NiagaraComponent.SetVariableVec3` (`self.Small Laser FX`) "User.Beam_End" (`KismetMathLibrary.MakeVector` _distance))
          (if (`self.CanDamage?`)
            (bind _asbp_ursadeath_player (cast `/Game/Ursadeath/PlayerCharacter/Blueprints/BP_UrsadeathPlayer` _hitactor))
            (if (<= (`self.Cooldown_Tracker`) 0.0)
              (`UDPlayerCharacter.DamagePlayer` _asbp_ursadeath_player (`self.Damage`))
              (set `self.Cooldown_Tracker` (`self.Cooldown`)))))))))

(event `Shoot`
  ;[1 1 1] Shoot Event
  (`BlackboardComponent.SetValueAsBool` (`AIBlueprintHelperLibrary.GetBlackboard` null) "IsFiring?" true)
  (set `self.LazerIsFiring?` true)
  (`self.Small Lazer Knowledge`)
  (`AudioComponent.Play` (`self.AudioChargingLaser`) 0.0)
  (`Timeline|TL_LaserStartup` :!via `PlayFromStart`
    (:`Finished`
      (`AudioComponent.Stop` (`self.AudioChargingLaser`))
      (set `self.bUseControllerRotationYaw` false)
      (`self.Large Lazer Knowledge`)
      (`AudioComponent.Play` (`self.AudioFiringLaser`) 0.0)
      (set `self.CanDamage?` true)
      (`KismetSystemLibrary.Delay` 3.0)
      (`ActorComponent.Deactivate` (`self.Laser FX`))
      (set `self.bUseControllerRotationYaw` true)
      (set `self.CanDamage?` false)
      (set `self.LazerIsFiring?` false)
      (`BlackboardComponent.SetValueAsBool` (`AIBlueprintHelperLibrary.GetBlackboard` null) "IsFiring?" false)
      (`BlackboardComponent.SetValueAsBool` (`AIBlueprintHelperLibrary.GetBlackboard` null) "LazerAimed" false)
      (`AudioComponent.Stop` (`self.AudioFiringLaser`)))))

(event `Large Lazer Knowledge`
  ;[1 1 1] Large Lazer Knowledge
  (`ActorComponent.Activate` (`self.Laser FX`) true)
  (`ActorComponent.Deactivate` (`self.Small Laser FX`)))

(event `Small Lazer Knowledge`
  ;[1 1 1] Small Lazer Knowledge
  (if (not (`BlackboardComponent.GetValueAsBool` (`AIBlueprintHelperLibrary.GetBlackboard` null) "NoFire"))
    (`ActorComponent.Activate` (`self.Small Laser FX`) true)))

(event `self.OnInterrupted`
  (params (WasAlreadyStunned :type Boolean))
  ;[1 1 1] Stop the laser when the enemy is stunned.
  (if (not WasAlreadyStunned)
    (`TimelineComponent.Stop` (`self.TL_LaserStartup`))
    (`ActorComponent.Deactivate` (`self.Small Laser FX`))
    (`ActorComponent.Deactivate` (`self.Laser FX`))
    (set `self.CanDamage?` false)
    (set `self.LazerIsFiring?` false)
    (`BlackboardComponent.SetValueAsBool` (`AIBlueprintHelperLibrary.GetBlackboard` null) "IsFiring?" false)
    (`AudioComponent.Stop` (`self.AudioFiringLaser`))
    (`AudioComponent.Stop` (`self.AudioChargingLaser`))
    (`BlackboardComponent.SetValueAsBool` (`AIBlueprintHelperLibrary.GetBlackboard` null) "LazerAimed" false)))

(event `self.AIPerception.OnTargetPerceptionUpdated`
  (params (Actor :type "Actor Object Reference") (Stimulus :type "AIStimulus Structure"))
  (bind _returnvalue (`AIBlueprintHelperLibrary.GetBlackboard` null))
  ;[1 1 1] AI Perception (Checking to see if enemy has eye contact with the player or not)
  (cast `/Game/Ursadeath/PlayerCharacter/Blueprints/BP_UrsadeathPlayer` Actor)
  (`/Engine/EditorBlueprintResources/StandardMacros.IsValid` _returnvalue
    (:`Is Valid`
      (`BlackboardComponent.SetValueAsBool` _returnvalue "CanSeePlayer?" Stimulus_bSuccessfullySensed))))

(fn `UserConstructionScript`)