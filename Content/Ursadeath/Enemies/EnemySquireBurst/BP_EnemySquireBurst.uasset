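; Burst-fire squire enemy that shoots projectiles at the Ursadeath player.
; When its spawn sequence ends it sets the blackboard "CanSeePlayer?" flag to true.
; AI Perception updates then set that flag from whether the player is successfully sensed.
; Shoot spawns three BP_BurstKnightProjectile actors from the Arrow's transform, spaced by short delays.
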(event `self.OnSpawnSequenceEnd`
  ;[1 1 1] Setting CanSeePlayer to be true once spawned
  (`BlackboardComponent.SetValueAsBool` (`AIBlueprintHelperLibrary.GetBlackboard` null) "CanSeePlayer?" true))

(event `Shoot`
  ;[1 1 1] Shooting Fireball
  (`|SpawnActorFromClass` "/Game/Ursadeath/Enemies/EnemyKnightBurst/BP_BurstKnightProjectile.BP_BurstKnightProjectile_C" (`SceneComponent.K2_GetComponentToWorld` (`self.Arrow`)) "AlwaysSpawn" "MultiplyWithRoot" null null)
  (`KismetSystemLibrary.Delay` 0.5)
  (`|SpawnActorFromClass` "/Game/Ursadeath/Enemies/EnemyKnightBurst/BP_BurstKnightProjectile.BP_BurstKnightProjectile_C" (`SceneComponent.K2_GetComponentToWorld` (`self.Arrow`)) "AlwaysSpawn" "MultiplyWithRoot" null null)
  (`KismetSystemLibrary.Delay` 0.5)
  (`|SpawnActorFromClass` "/Game/Ursadeath/Enemies/EnemyKnightBurst/BP_BurstKnightProjectile.BP_BurstKnightProjectile_C" (`SceneComponent.K2_GetComponentToWorld` (`self.Arrow`)) "AlwaysSpawn" "MultiplyWithRoot" null null))

(event `self.AIPerception.OnTargetPerceptionUpdated`
  (params (Actor :type "Actor Object Reference") (Stimulus :type "AIStimulus Structure"))
  ;[1 1 1] Checking whether the Enemy can see the player
  (cast `/Game/Ursadeath/PlayerCharacter/Blueprints/BP_UrsadeathPlayer` Actor)
  (`BlackboardComponent.SetValueAsBool` (`AIBlueprintHelperLibrary.GetBlackboard` null) "CanSeePlayer?" Stimulus_bSuccessfullySensed))

(fn `UserConstructionScript`)