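; Laser-firing Squire enemy that telegraphs a beam, then damages the player it hits.
; Shoot shows a small aiming beam during a startup timeline, then locks controller yaw and fires the large damaging beam for a fixed duration.
; While firing, Tick sphere-traces forward to set Niagara beam length and apply cooldown-gated damage.
; Perception and spawn completion update blackboard sight, firing state is mirrored there, and a stun cancels the laser.
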(event `self.OnSpawnSequenceEnd`
  (`BlackboardComponent.SetValueAsBool` (`AIBlueprintHelperLibrary.GetBlackboard` null) "CanSeePlayer?" true))

(event `self.ReceiveBeginPlay`
  (`ActorComponent.Deactivate` (`self.Laser FX`))
  (`ActorComponent.Deactivate` (`self.Small Laser FX`)))

(event `self.ReceiveTick`
  (params (DeltaSeconds :type "Float (single-precision)"))
  (bind _weapon_attack_spawn (`self.Weapon Attack Spawn`))
  (bind _returnvalue (`SceneComponent.K2_GetComponentLocation` _weapon_attack_spawn))
  (`|ExecutionSequence`
    (:`then_0`
      (if (> (`self.Cooldown_Tracker`) 0.0)
        (set `self.Cooldown_Tracker` (- (`self.Cooldown_Tracker`) DeltaSeconds))))
    (:`then_1`
      (if (`self.LazerIsFiring?`)
        (bind _outhit (`KismetSystemLibrary.SphereTraceSingleForObjects` _returnvalue (+ _returnvalue (* (`SceneComponent.GetForwardVector` _weapon_attack_spawn) 10000.0)) 20.0 (`|MakeArray` "ObjectTypeQuery1" "ObjectTypeQuery8" :!type "EObjectTypeQuery Enum")))
        (bind (_bblockinghit _binitialoverlap _time _distance _location _impactpoint _normal _impactnormal _physmat _hitactor) (`GameplayStatics.BreakHitResult` _outhit))
        (if _bblockinghit
          (`NiagaraComponent.SetVariableVec3` (`self.Laser FX`) "User.Beam_End" (`KismetMathLibrary.MakeVector` _distance))
          (`NiagaraComponent.SetVariableVec3` (`self.Small Laser FX`) "User.Beam_End" (`KismetMathLibrary.MakeVector` _distance))
          (`KismetSystemLibrary.PrintString` (`KismetSystemLibrary.GetDisplayName` _hitactor))
          (if (`self.CanDamage?`)
            (bind _asbp_ursadeath_player (cast `/Game/Ursadeath/PlayerCharacter/Blueprints/BP_UrsadeathPlayer` _hitactor))
            (if (<= (`self.Cooldown_Tracker`) 0.0)
              (`UDPlayerCharacter.DamagePlayer` _asbp_ursadeath_player (`self.Damage`))
              (`KismetSystemLibrary.PrintString` "Lazer Hit!")
              (set `self.Cooldown_Tracker` (`self.Cooldown`)))))))))

(event `Shoot`
  (`BlackboardComponent.SetValueAsBool` (`AIBlueprintHelperLibrary.GetBlackboard` null) "IsFiring?" true)
  (set `self.LazerIsFiring?` true)
  (`self.Small Lazer Knowledge`)
  (`Timeline|TL_LaserStartup` :!via `PlayFromStart`
    (:`Finished`
      (set `self.bUseControllerRotationYaw` false)
      (`self.Large Lazer Knowledge`)
      (set `self.CanDamage?` true)
      (`KismetSystemLibrary.Delay` 3.0)
      (`ActorComponent.Deactivate` (`self.Laser FX`))
      (set `self.bUseControllerRotationYaw` true)
      (set `self.CanDamage?` false)
      (set `self.LazerIsFiring?` false)
      (`BlackboardComponent.SetValueAsBool` (`AIBlueprintHelperLibrary.GetBlackboard` null) "IsFiring?" false))))

(event `Large Lazer Knowledge`
  (`ActorComponent.Activate` (`self.Laser FX`) true)
  (`ActorComponent.Deactivate` (`self.Small Laser FX`)))

(event `Small Lazer Knowledge`
  (`ActorComponent.Activate` (`self.Small Laser FX`) true))

(event `self.OnStunned`
  (params (WasAlreadyStunned :type Boolean))
  (if (not WasAlreadyStunned)
    ;[1 1 1] Stop the laser when the enemy is stunned.
    (`TimelineComponent.Stop` (`self.TL_LaserStartup`))
    (`ActorComponent.Deactivate` (`self.Small Laser FX`))
    (`ActorComponent.Deactivate` (`self.Laser FX`))
    (set `self.CanDamage?` false)
    (set `self.LazerIsFiring?` false)
    (`BlackboardComponent.SetValueAsBool` (`AIBlueprintHelperLibrary.GetBlackboard` null) "IsFiring?" false)))

(event `self.AIPerception.OnTargetPerceptionUpdated`
  (params (Actor :type "Actor Object Reference") (Stimulus :type "AIStimulus Structure"))
  (cast `/Game/Ursadeath/PlayerCharacter/Blueprints/BP_UrsadeathPlayer` Actor)
  (`BlackboardComponent.SetValueAsBool` (`AIBlueprintHelperLibrary.GetBlackboard` null) "CanSeePlayer?" Stimulus_bSuccessfullySensed))

(fn `UserConstructionScript`)