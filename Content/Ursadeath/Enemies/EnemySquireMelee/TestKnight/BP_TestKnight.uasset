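; Test knight enemy, in the melee squire folder, that reacts to incoming attacks and hurts the player on contact.
; On BeginPlay it binds the attack-received event to apply a slow on any damage or stun, then boost rocket hits' damage and stun time as a weakness.
; A sphere overlap damages the player while circle damage is enabled and the knight is not stunned.
; An older movement-stopping slow remains as unreachable nodes.
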(event `self.ReceiveBeginPlay`
  (`parent.ReceiveBeginPlay`)
  (add `self.OnAttackRecieved` (delegate `Damage Weaknesses`)))

(event `Damage Weaknesses` :!signature `self.OnAttackRecieved`
  (params (DamageData :type "UDPlayerAttackData Object Reference"))
  (bind (_attackstats_attacktype _attackstats_damage _attackstats_stuntime) (break `PlayerAttackStats` (`UDPlayerAttackData.AttackStats` DamageData)))
  (bind (_attackstats_attacktype_2 _attackstats_damage_2 _attackstats_stuntime_2) (break `PlayerAttackStats` (`UDPlayerAttackData.AttackStats` DamageData)))
  (`|ExecutionSequence`
    (:`then_0`
      (if (or (> _attackstats_damage 0) (> _attackstats_stuntime 0.0))
        (`self.ApplySlow` (`self.Slow Time`))))
    (:`then_1`
      ;[1 1 1] Rocket Weakness
      (if (`|EnumEquality` _attackstats_attacktype_2 "ROCKET")
        (`UDPlayerAttackData.SetDamage` DamageData (`KismetMathLibrary.FTrunc` (* _attackstats_damage_2 1.5)))
        (`UDPlayerAttackData.SetStunTime` DamageData (+ _attackstats_stuntime_2 (`self.Rocket Stun Time`)))))))

(event `self.Sphere1.OnComponentBeginOverlap`
  (params (OverlappedComponent :type "PrimitiveComponent Object Reference") (OtherActor :type "Actor Object Reference") (OtherComp :type "PrimitiveComponent Object Reference") (OtherBodyIndex :type Integer) (bFromSweep :type Boolean) (SweepResult :type "HitResult Structure (by ref)"))
  (if (and (`self.CanDamageCircle`) (!= (`self.IsStunned`) true))
    (bind _asbp_ursadeath_player (cast `/Game/Ursadeath/PlayerCharacter/Blueprints/BP_UrsadeathPlayer` OtherActor))
    (`UDPlayerCharacter.DamagePlayer` _asbp_ursadeath_player (`self.Damage`))))

(event `self.ReceiveTick`
  (params (DeltaSeconds :type "Float (single-precision)"))
  (`parent.ReceiveTick` DeltaSeconds))

(fn `UserConstructionScript`
  (`parent.UserConstructionScript`))