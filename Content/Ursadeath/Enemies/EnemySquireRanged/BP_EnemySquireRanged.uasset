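; BP_EnemySquireRanged is a ranged squire enemy in Ursadeath that fires projectiles.
; AI perception writes the blackboard key "CanSeePlayer?" whenever the player's stimulus updates.
; When the spawn sequence ends, it seeds that key by checking whether sight currently perceives the player.
; Its Shoot event spawns a BP_ProjectileBase at the Arrow component's transform and plays a fireball sound at the enemy's location.
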(event `self.OnSpawnSequenceEnd`
  (`BlackboardComponent.SetValueAsBool` (`AIBlueprintHelperLibrary.GetBlackboard` null) "CanSeePlayer?" (`KismetArrayLibrary.Array_Contains` (`AIPerceptionComponent.GetCurrentlyPerceivedActors` (`self.AIPerception`) "/Script/AIModule.AISense_Sight") (`UDPlayerCharacter.GetCharacterInPlay`))))

(event `self.ReceiveTick`
  (params (DeltaSeconds :type "Float (single-precision)")))

(event `Shoot`
  (`|SpawnActorFromClass` "/Game/Ursadeath/Enemies/Core/Blueprints/BP_ProjectileBase.BP_ProjectileBase_C" (`SceneComponent.K2_GetComponentToWorld` (`self.Arrow`)) "AlwaysSpawn" "MultiplyWithRoot" null null)
  (`GameplayStatics.PlaySoundAtLocation` "/Game/Ursadeath/Enemies/EnemySquireRanged/UD_EnemyFireball.UD_EnemyFireball" (`self.K2_GetActorLocation`) (struct) 1.0 1.0 0.0 null null null null))

(event `self.AIPerception.OnTargetPerceptionUpdated`
  (params (Actor :type "Actor Object Reference") (Stimulus :type "AIStimulus Structure"))
  (cast `/Game/Ursadeath/PlayerCharacter/Blueprints/BP_UrsadeathPlayer` Actor)
  (`BlackboardComponent.SetValueAsBool` (`AIBlueprintHelperLibrary.GetBlackboard` null) "CanSeePlayer?" Stimulus_bSuccessfullySensed))

(fn `UserConstructionScript`)