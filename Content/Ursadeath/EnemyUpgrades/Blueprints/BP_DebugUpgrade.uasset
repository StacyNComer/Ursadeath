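; BP_DebugUpgrade is a debug enemy upgrade for Ursadeath that prints upgrade activity to screen and log.
; When applied, it prints a fixed confirmation message.
; Its OnEnemyDataChangeApplied override prints the incoming enemy data, including class, icons, description and spawn scalar, then returns the parent implementation's result without altering the data itself.
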(event `self.OnUpgradeApplied`
  (params (Enemy :type "UDEnemy Object Reference"))
  (`KismetSystemLibrary.PrintString` "I am an upgrage!"))

(fn `OnEnemyDataChangeApplied`
  (params (OriginalData :type "EnemySpawnData Structure"))
  (returns (ReturnValue :type "EnemySpawnData Structure"))
  (bind (_enemyclass _enemyicon _upgradeicon _description _spawnscalar) (break `EnemySpawnData` OriginalData))
  (`|ExecutionSequence`
    (:`then_0`
      (`KismetSystemLibrary.PrintString` (`KismetSystemLibrary.GetClassDisplayName` _enemyclass)))
    (:`then_1`
      (`KismetSystemLibrary.PrintString` (`KismetSystemLibrary.GetDisplayName` _enemyicon)))
    (:`then_2`
      (`KismetSystemLibrary.PrintString` (`KismetSystemLibrary.GetDisplayName` _upgradeicon)))
    (:`then_3`
      (`KismetSystemLibrary.PrintString` (`KismetTextLibrary.Conv_TextToString` (break `UIDescription` _description))))
    (:`then_4`
      (`KismetSystemLibrary.PrintString` (`KismetTextLibrary.Conv_TextToString` (`.Body` (break `UIDescription` _description)))))
    (:`then_5`
      (`KismetSystemLibrary.PrintString` (`KismetStringLibrary.Conv_IntToString` _spawnscalar)))
    (:`then_6`
      (bind _returnvalue (`parent.OnEnemyDataChangeApplied` OriginalData))
      (return _returnvalue))))