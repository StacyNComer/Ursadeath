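; Health pickup that hides itself when used and reappears on respawn, driven by inherited or external pickup events.
; Use and respawn toggle the HealthSphere's visibility and collision instead of destroying the actor, each spawning its own Niagara effect.
; Tick spins the heart by a fixed step each frame, independent of delta time.
; Respawn indicator widget logic is present but disconnected, so cooldown ticks do nothing here.
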(event `self.OnPickupUsed`
  ;[1 1 1] Make the pickup invisible and intangable when used. The pickup disappears when used instead of being destroyed.
  (`SceneComponent.SetVisibility` (`self.Health Sphere`) false true)
  (`PrimitiveComponent.SetCollisionEnabled` (`self.Health Sphere`) "NoCollision")
  (`NiagaraFunctionLibrary.SpawnSystemAtLocation` "/Game/Ursadeath/MapFeatures/HealthPickup/FX/NS_HealthPickupCollected.NS_HealthPickupCollected" (`SceneComponent.K2_GetComponentLocation` (`self.Health Sphere`))))

(event `self.OnPickupRespawned`
  ;[1 1 1] When the pickup "respawns", make it visible and restore its collision. The pickup disappears when used instead of being destroyed.
  (`SceneComponent.SetVisibility` (`self.Health Sphere`) true true)
  (`PrimitiveComponent.SetCollisionEnabled` (`self.Health Sphere`) "QueryAndPhysics")
  (`NiagaraFunctionLibrary.SpawnSystemAtLocation` "/Game/Ursadeath/MapFeatures/HealthPickup/FX/NS_HealthPickupSpawn.NS_HealthPickupSpawn" (`self.K2_GetActorLocation`)))

(event `self.ReceiveTick`
  (params (DeltaSeconds :type "Float (single-precision)"))
  ;[1 1 1] Rotate the heart
  (`SceneComponent.K2_AddWorldRotation` (`self.Heart`) (struct :`Yaw` 1.0) false false))

(event `self.OnCooldownTick`
  (params (CooldownMax :type "Float (single-precision)") (CooldownRemaining :type "Float (single-precision)")))

(event `self.ReceiveBeginPlay`)

(fn `UserConstructionScript`)