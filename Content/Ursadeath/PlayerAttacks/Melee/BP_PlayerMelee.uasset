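; Short-lived player melee attack actor that resolves one hit as soon as it spawns.
; On BeginPlay it sphere-traces for pawns along its forward vector, using its melee range and cast radius and ignoring its owner.
; If the single trace result is a UDEnemy, it applies its attack stats to that enemy.
; The actor then destroys itself, so it has no tick or lingering hitbox.
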(event `self.ReceiveBeginPlay`
  (bind _returnvalue (`self.K2_GetActorLocation`))
  (bind _outhit (`KismetSystemLibrary.SphereTraceSingleForObjects` _returnvalue (+ (* (`self.GetActorForwardVector`) (`self.Melee Range`)) _returnvalue) (`self.Melee Cast Radius`) (`|MakeArray` "ObjectTypeQuery3" :!type "EObjectTypeQuery Enum") true (`|MakeArray` (`self.GetOwner`)) "None" true (struct :`R` 1.0 :`A` 1.0) (struct :`G` 1.0 :`A` 1.0) 0.5))
  (bind _asudenemy (cast `UDEnemy` (`.HitActor` (`GameplayStatics.BreakHitResult` _outhit)))
    (:`then`
      (`self.ApplyAttackToEnemy` _asudenemy (`self.AttackStats`)))
    (:`CastFailed`
      _))
  (`self.K2_DestroyActor`))

(fn `UserConstructionScript`)