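; Player shockwave attack actor for Ursadeath that damages enemies and clears enemy projectiles in a straight horizontal path.
; On BeginPlay it keeps only its yaw, then runs a single long forward box multi-trace sized by ShockwaveSize, ignoring its owner.
; UDEnemy hits receive AttackStats through ApplyAttackToEnemy, while any other hit actor is assumed to be an enemy projectile and destroyed.
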(event `self.ReceiveBeginPlay`
  (bind (_returnvalue_roll _returnvalue_pitch _returnvalue_yaw) (`KismetMathLibrary.BreakRotator` (`self.K2_GetActorRotation`)))
  (bind _shockwave_size (`self.Shockwave Size`))
  (`self.K2_SetActorRotation` (`KismetMathLibrary.MakeRotator` 0.0 0.0 _returnvalue_yaw))
  (bind _outhits (`KismetSystemLibrary.BoxTraceMultiForObjects` (`self.K2_GetActorLocation`) (+ (* (`KismetMathLibrary.ProjectVectorOnToPlane` (`self.GetActorForwardVector`) (0.0 0.0 1.0)) 4000.0) (`self.K2_GetActorLocation`)) (`KismetMathLibrary.MakeVector` _shockwave_size _shockwave_size _shockwave_size) (`self.K2_GetActorRotation`) (`|MakeArray` "ObjectTypeQuery10" "ObjectTypeQuery9" :!type "EObjectTypeQuery Enum") false (`|MakeArray` (`self.GetOwner`)) "None" true (struct :`R` 1.0 :`A` 1.0) (struct :`G` 1.0 :`A` 1.0) 1.0))
  (for _array_element _outhits
    (bind _asudenemy (cast `UDEnemy` (`.HitActor` (`GameplayStatics.BreakHitResult` _array_element)))
      (:`then`
        (`self.ApplyAttackToEnemy` _asudenemy (`self.AttackStats`)))
      (:`CastFailed`
        (`self.K2_DestroyActor` (`.HitActor` (`GameplayStatics.BreakHitResult` _array_element))) ; If we didn't hit an enemy, that means we hit an Enemy Projectile.
      ))))

(fn `UserConstructionScript`)