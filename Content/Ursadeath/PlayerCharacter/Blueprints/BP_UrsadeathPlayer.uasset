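; BP_UrsadeathPlayer is the player character Blueprint for Ursadeath, and its only live logic lets a controller move the mouse cursor.
; The IA_ControllerCursor input is scaled per axis and by viewport size, Y is inverted, and the rounded result is added to the current mouse position.
; BeginPlay, Tick and the construction script are empty, and leftover settings-reset and linked-button print nodes are disconnected.
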(event `self.ReceiveBeginPlay`)

(event `EnhancedInput|/Game/Ursadeath/PlayerCharacter/Input/Actions/UI/IA_ControllerCursor`
  (params (ActionValue :type "Vector2D Structure") (ElapsedSeconds :type "Float (double-precision)") (TriggeredSeconds :type "Float (double-precision)") (InputAction :type "InputAction Object Reference" :default "/Game/Ursadeath/PlayerCharacter/Input/Actions/UI/IA_ControllerCursor.IA_ControllerCursor"))
  (bind _returnvalue (`GameplayStatics.GetPlayerController` 0))
  (bind (_locationx _locationy) (`PlayerController.GetMousePosition` _returnvalue))
  (bind (_returnvalue_x _returnvalue_y) (`KismetMathLibrary.BreakVector2D` (* ActionValue (3.0 5.0) (/ (`WidgetLayoutLibrary.GetViewportSize`) (1000.0 1000.0)))))
  (:`Triggered`
    (`PlayerController.SetMouseLocation` _returnvalue (`KismetMathLibrary.Round` (+ _returnvalue_x _locationx)) (`KismetMathLibrary.Round` (+ (* _returnvalue_y -1) _locationy)))))

(event `self.ReceiveTick`
  (params (DeltaSeconds :type "Float (single-precision)")))

(event `EnhancedInput|/Game/Ursadeath/PlayerCharacter/Input/Actions/UI/IA_ControllerUIClick`
  (params (ActionValue :type Boolean) (ElapsedSeconds :type "Float (double-precision)") (TriggeredSeconds :type "Float (double-precision)") (InputAction :type "InputAction Object Reference" :default "/Game/Ursadeath/PlayerCharacter/Input/Actions/UI/IA_ControllerUIClick.IA_ControllerUIClick")))

(event `Key|P` :paused true
  (params (Key :type "Key Structure")))

(fn `UserConstructionScript`)