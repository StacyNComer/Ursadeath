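; Player upgrade that rewards melee kills with haste and healing.
; When added, it binds its effect to the owning player's enemy-hit event and filters for melee hits that kill the enemy.
; Every such kill applies a short haste, while health is restored by the heal amount only if the victim is not a Squire-tier enemy.
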(event `self.OnUpgradeAdded`
  (params (Player :type "UDPlayerCharacter Object Reference"))
  (add `UDPlayerCharacter.OnEnemyHit` (`self.OwningPlayer`) (delegate `Upgrade Effect`)))

(event `Upgrade Effect`
  (params (HitData :type "EnemyHitData Structure"))
  (bind _attackstats_attacktype (break `PlayerAttackStats` (`UDPlayerAttack.AttackStats` HitData_Attack)))
  (if (and HitData_EnemyWasKilled (`|EnumEquality` _attackstats_attacktype "MELEE"))
    (`UDPlayerCharacter.ApplyHaste` (`self.OwningPlayer`) 2.5)
    (if (`|EnumInequality` HitData_EnemyTier "SQUIRE")
      (`UDPlayerCharacter.RestoreHealth` (`self.OwningPlayer`) (`self.Heal Amount`)))))