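; BP_UpgradeTest is a test upgrade for the player that rewards melee kills with healing.
; When added, it binds its effect to the owning player's enemy death event and immediately damages that player.
; On each enemy death, the effect prints the attack type from the hit data and restores a fixed amount of health if the attack was melee.
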(event `self.OnUpgradeAdded`
  (add `UDPlayerCharacter.OnEnemyDeath` (`self.OwningPlayer`) (delegate `Upgrade Effect`))
  (`UDPlayerCharacter.DamagePlayer` (`self.OwningPlayer`) 34))

(event `Upgrade Effect`
  (params (HitData :type "EnemyHitData Structure"))
  (bind _attackstats_attacktype (break `PlayerAttackStats` (`UDPlayerAttack.AttackStats` HitData_Attack)))
  (`KismetSystemLibrary.PrintString` null (`|GetEnumeratorNameAsString` _attackstats_attacktype))
  (if (`|EnumEquality` _attackstats_attacktype "MELEE")
    (`UDPlayerCharacter.RestoreHealth` (`self.OwningPlayer`) 25)))