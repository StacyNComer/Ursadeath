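; Player upgrade that makes rocket hits spawn a horizontal beam, damaging enemies in its path.
; Binds to the owning player's projectile-hit event, then spawns a Niagara beam at the rocket along its yaw.
; A sphere trace spanning the arena diameter applies the rocket's direct-hit attack to enemies, ignoring the actor originally hit.
; Visual and trace share BeamRadius, but the visual's length is hardcoded separately.
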(event `self.OnUpgradeAdded`
  (params (Player :type "UDPlayerCharacter Object Reference"))
  (add `UDPlayerCharacter.OnPlayerProjectileHit` (`self.OwningPlayer`) (delegate `Spawn Bomb Beam`)))

(event `Spawn Bomb Beam`
  (params (ProjectileHitData :type "PlayerProjectileHitData Structure"))
  (bind (_returnvalue_roll _returnvalue_pitch _returnvalue_yaw) (`KismetMathLibrary.BreakRotator` (`Actor.K2_GetActorRotation` ProjectileHitData_Projectile)))
  (bind (_returnvalue_roll_2 _returnvalue_pitch_2 _returnvalue_yaw_2) (`KismetMathLibrary.BreakRotator` (`Actor.K2_GetActorRotation` ProjectileHitData_Projectile)))
  (bind _returnvalue (`Actor.K2_GetActorLocation` ProjectileHitData_Projectile))
  (bind _attackstats_attacktype (break `PlayerAttackStats` (`UDPlayerAttack.AttackStats` ProjectileHitData_Projectile)))
  (if (`|EnumEquality` _attackstats_attacktype "ROCKET")
    ;[1 1 1] Spawn the beam's particle FX
    (bind _returnvalue_2 (`NiagaraFunctionLibrary.SpawnSystemAtLocation` "/Game/Ursadeath/Upgrades/Core/ParticleFX/NS_Beam.NS_Beam" (`Actor.K2_GetActorLocation` ProjectileHitData_Projectile) (`KismetMathLibrary.MakeRotator` 0.0 0.0 _returnvalue_yaw_2)))
    (`FXSystemComponent.SetVectorParameter` _returnvalue_2 "User.BeamEnd" (3000.0 0.0 0.0))
    (`FXSystemComponent.SetFloatParameter` _returnvalue_2 "User.Beam_Radius" (`self.Beam Radius`))
    ;[1 1 1] Damage each enemy caught in the beam. The beam's damage uses the rocket's direct hit damage!
    (bind _outhits (`KismetSystemLibrary.SphereTraceMultiForObjects` _returnvalue (+ _returnvalue (* (`KismetMathLibrary.GreaterGreater_VectorRotator` (1.0 0.0 0.0) (`KismetMathLibrary.MakeRotator` 0.0 0.0 _returnvalue_yaw)) (`UDCoreLibrary.GetArenaDiameter`))) (`self.Beam Radius`) (`|MakeArray` "ObjectTypeQuery10" :!type "EObjectTypeQuery Enum") false (`|MakeArray` ProjectileHitData_ActorHit)))
    (for _array_element _outhits
      (bind _asudenemy (cast `UDEnemy` (`.HitActor` (`GameplayStatics.BreakHitResult` _array_element))))
      (`UDPlayerAttack.ApplyAttackExclusive` ProjectileHitData_Projectile _asudenemy (`UDPlayerAttack.AttackStats` ProjectileHitData_Projectile) 1.0))))