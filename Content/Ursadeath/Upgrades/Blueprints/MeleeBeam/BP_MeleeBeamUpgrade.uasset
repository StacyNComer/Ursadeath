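; Player upgrade that turns the next melee attack after a shockwave into a long-range beam.
; Listens to spawned attacks: a shockwave arms the beam, shows its HUD icon and forces the melee cooldown to zero.
; An armed melee attack gains multiplied damage and extra stun, then sphere-traces forward to hit an enemy.
; It spawns a Niagara beam sized by the trace, then hides the icon and disarms.
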(event `self.OnUpgradeAdded`
  (params (Player :type "UDPlayerCharacter Object Reference"))
  (`|ExecutionSequence`
    (:`then_0`
      ;[1 1 1] Add the upgrade's icon to the player's HUD.
      (bind _returnvalue (`UDPlayerHUDWidget.AddPlayerStatusIcon` (`UDPlayerCharacter.HUDWidget` Player)))
      (bind _output_get (set `self.Upgrade Status Icon` _returnvalue))
      (`UDPlayerStatusIcon.SetStatusImage` _output_get "/Engine/EditorResources/Ai_Spawnpoint.Ai_Spawnpoint")
      (`Widget.SetVisibility` (`UDPlayerStatusIcon.StatusCounter` _output_get) "Collapsed"))
    (:`then_1`
      (add `UDPlayerCharacter.OnAttackSpawned` Player (delegate `Ready Melee Beam`)))
    (:`then_2`
      (add `UDPlayerCharacter.OnAttackSpawned` Player (delegate `Spawn Melee Beam`)))))

(event `Ready Melee Beam`
  (params (AttackActor :type "UDPlayerAttack Object Reference"))
  (bind _attackstats_attacktype (break `PlayerAttackStats` (`UDPlayerAttack.AttackStats` AttackActor)))
  (if (and (`|EnumEquality` _attackstats_attacktype "SHOCKWAVE") (not (`self.MeleeBeamReady`)))
    (set `self.MeleeBeamReady` true)
    (`Widget.SetVisibility` (`self.Upgrade Status Icon`) "Visible")
    (`UDPlayerCooldownAbility.ForceCooldown` (`UDPlayerCharacter.MeleeAbility` (`self.OwningPlayer`)) 0.0)))

(event `Spawn Melee Beam`
  (params (AttackActor :type "UDPlayerAttack Object Reference"))
  (bind _attackstats_attacktype (break `PlayerAttackStats` (`UDPlayerAttack.AttackStats` AttackActor)))
  (bind (_attackstats_attacktype_2 _attackstats_damage _attackstats_stuntime) (break `PlayerAttackStats` (`UDPlayerAttack.AttackStats` AttackActor)))
  (bind _attackspawncomponent (`UDPlayerCharacter.AttackSpawnComponent` (`self.OwningPlayer`)))
  (bind _attackspawncomponent_2 (`UDPlayerCharacter.AttackSpawnComponent` (`self.OwningPlayer`)))
  (bind (_returnvalue_roll _returnvalue_pitch _returnvalue_yaw) (`KismetMathLibrary.BreakRotator` (`SceneComponent.K2_GetComponentRotation` _attackspawncomponent)))
  (bind _returnvalue (`SceneComponent.K2_GetComponentLocation` _attackspawncomponent_2))
  (if (and (`|EnumEquality` _attackstats_attacktype "MELEE") (`self.MeleeBeamReady`))
    (`|ExecutionSequence`
      (:`then_0`
        ;[1 1 1] Perform a sphere trace for an enemy and damage them if one was hit
        (set `UDPlayerAttack.AttackStats` (make `PlayerAttackStats` _attackstats_attacktype_2 (* _attackstats_damage (`self.Beam Damage Multiplier`)) (+ _attackstats_stuntime (`self.Beam Stun`))) AttackActor)
        (bind (_outhit _returnvalue_2) (`KismetSystemLibrary.SphereTraceSingleForObjects` :`Start` _returnvalue :`End` (+ _returnvalue (* (`SceneComponent.GetForwardVector` _attackspawncomponent_2) 3000)) :`Radius` (`self.Beam Radius`) :`ObjectTypes` (`|MakeArray` "ObjectTypeQuery10" :!type "EObjectTypeQuery Enum") :`DrawTime` 2.0))
        (if _returnvalue_2
          (bind _asudenemy (cast `UDEnemy` (`.HitActor` (`GameplayStatics.BreakHitResult` _outhit))))
          (`UDPlayerAttack.ApplyAttackExclusive` AttackActor _asudenemy (`UDPlayerAttack.AttackStats` AttackActor) 1.0)))
      (:`then_1`
        ;[1 1 1] Spawn the beam's particle FX
        (bind _returnvalue_3 (`NiagaraFunctionLibrary.SpawnSystemAtLocation` "/Game/Ursadeath/Upgrades/Core/ParticleFX/NS_Beam.NS_Beam" (`SceneComponent.K2_GetComponentLocation` _attackspawncomponent) (`KismetMathLibrary.MakeRotator` 0.0 _returnvalue_pitch _returnvalue_yaw)))
        (`FXSystemComponent.SetVectorParameter` _returnvalue_3 "User.Beam_End" (`KismetMathLibrary.MakeVector` (`KismetMathLibrary.SelectFloat` (`.Distance` (`GameplayStatics.BreakHitResult` _outhit)) 6000.0 _returnvalue_2)))
        (`FXSystemComponent.SetFloatParameter` _returnvalue_3 "User.Beam_Width" (`self.Beam Radius`))
        (`NiagaraComponent.SetVariableLinearColor` _returnvalue_3 "User.Beam_Color" (`self.Beam Color`)))
      (:`then_2`
        (`Widget.SetVisibility` (`self.Upgrade Status Icon`) "Collapsed")
        (set `self.MeleeBeamReady` false)))))