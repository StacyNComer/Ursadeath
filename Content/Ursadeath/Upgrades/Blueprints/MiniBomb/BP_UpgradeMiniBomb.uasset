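; Player upgrade that spawns a mini bomb attack after enough primary fire attacks.
; It binds to the player's attack-spawned event and counts primary fire, adding a multiplied amount per attack while Frenzied.
; Once the count has reached the requirement, the next primary attack resets it and spawns BP_PlayerMiniBomb from the player.
; A HUD status icon mirrors the counter, reusing the status time bar to show charge progress.
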(event `self.OnUpgradeAdded`
  (params (Player :type "UDPlayerCharacter Object Reference"))
  (`|ExecutionSequence`
    (:`then_0`
      (bind _returnvalue (`UDPlayerHUDWidget.AddPlayerStatusIcon` (`UDPlayerCharacter.HUDWidget` Player)))
      (bind _output_get (set `self.Status Widget` _returnvalue))
      (set `UDPlayerStatusIcon.bDisappearWhenStatusDepleted` false _output_get)
      (set `UDPlayerStatusIcon.bCounterDisplaysStatusTime` true _output_get)
      (`UDPlayerStatusIcon.SetStatusCounterMinFractionalDigits` _output_get 0)
      (`UDPlayerStatusIcon.SetStatusImage` _output_get (`self.Status Icon`))
      (`Widget.SetVisibility` _output_get "Visible")
      (`UDPlayerStatusIcon.StartStatusBarFromTime` _output_get (`self.MinibombCountRequirement`) 0.0))
    (:`then_1`
      (add `UDPlayerCharacter.OnAttackSpawned` Player (delegate `MiniBomb Counter`)))))

(event `MiniBomb Counter`
  (params (AttackActor :type "UDPlayerAttack Object Reference"))
  (bind _attackstats_attacktype (break `PlayerAttackStats` (`UDPlayerAttack.AttackStats` AttackActor)))
  (bind _returnvalue (`KismetMathLibrary.SelectFloat` (`self.FrenzyCounterMultiplier`) 1.0 (`UDPlayerCharacter.IsFrenzied` (`self.OwningPlayer`))))
  (if (`|EnumEquality` _attackstats_attacktype "PRIMARY_FIRE")
    (if (>= (`self.PrimaryCounter`) (`self.MinibombCountRequirement`))
      (set `self.PrimaryCounter` 0.0)
      (`UDPlayerStatusIcon.SetStatusValue` (`self.Status Widget`) 0.0)
      (`UDPlayerCharacter.SpawnAttackFromPlayer` (`self.OwningPlayer`) "/Game/Ursadeath/Upgrades/Blueprints/MiniBomb/BP_PlayerMiniBomb.BP_PlayerMiniBomb_C")
      (else
        (set `self.PrimaryCounter` (+ (`self.PrimaryCounter`) _returnvalue))
        (`UDPlayerStatusIcon.AddStatusValue` (`self.Status Widget`) _returnvalue)))))