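; BP_PickupBombAttack is the explosion attack for the Pickup Bomb upgrade, damaging enemies around the point where it spawns.
; On BeginPlay it spawns the NS_PickupBombExplosion Niagara effect, then runs a sphere overlap of ExplosionRadius and applies AttackStats to each UDEnemy found.
; The node passing ExplosionRadius to the effect is disconnected, so the visual does not receive the gameplay radius.
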(event `self.ReceiveBeginPlay`
  (`|ExecutionSequence`
    (:`then_0`
      (`NiagaraFunctionLibrary.SpawnSystemAtLocation` "/Game/Ursadeath/Upgrades/Blueprints/PickupBomb/NS_PickupBombExplosion.NS_PickupBombExplosion" (`self.K2_GetActorLocation`)))
    (:`then_1`
      (bind _outactors (`KismetSystemLibrary.SphereOverlapActors` (`self.K2_GetActorLocation`) (`self.Explosion Radius`) (`|MakeArray` "ObjectTypeQuery10" :!type "EObjectTypeQuery Enum")))
      (for _array_element _outactors
        (bind _asudenemy (cast `UDEnemy` _array_element))
        (`self.ApplyAttackToEnemy` _asudenemy (`self.AttackStats`))))))

(fn `UserConstructionScript`)