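; Player upgrade that periodically turns melee attacks into a super punch with double damage and extra stun.
; Boosts melee attacks as they spawn while ready; cooldown starts only on hitting a non-Squire enemy, so pickups don't expend it.
; That hit also spawns a Niagara blast and reapplies the attack to enemies within the blast radius, without energy gain.
; Ticking drains the cooldown and HUD status bar, playing a sound on recharge.
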(event `self.OnUpgradeAdded`
  (params (Player :type "UDPlayerCharacter Object Reference"))
  (`|ExecutionSequence`
    (:`then_0`
      ;[1 1 1] Setup the HUD to show when the Super Melee is ready
      (bind _returnvalue (`UDPlayerHUDWidget.AddPlayerStatusIcon` (`UDPlayerCharacter.HUDWidget` Player)))
      (bind _output_get (set `self.Status Widget` _returnvalue))
      (set `UDPlayerStatusIcon.bDisappearWhenStatusDepleted` false _output_get)
      (set `UDPlayerStatusIcon.bHideCounterWhenStatusDepleted` true _output_get)
      (`UDPlayerStatusIcon.SetStatusImage` _output_get (`self.Status Icon`))
      (`Widget.SetVisibility` _output_get "Visible")
      (`Widget.SetVisibility` (`UDPlayerStatusIcon.GetStatusCounter` _output_get) "Collapsed"))
    (:`then_1`
      (add `UDPlayerCharacter.OnAttackSpawned` Player (delegate `Super Melee`)))
    (:`then_2`
      (add `UDPlayerCharacter.OnEnemyHit` Player (delegate `Set Super Punch Cooldown`)))))

(event `Super Melee`
  (params (AttackActor :type "UDPlayerAttack Object Reference"))
  (bind _attackstats_attacktype (break `PlayerAttackStats` (`UDPlayerAttack.AttackStats` AttackActor)))
  (bind (_attackstats_attacktype_2 _attackstats_damage _attackstats_stuntime) (break `PlayerAttackStats` (`UDPlayerAttack.AttackStats` AttackActor)))
  ;[1 1 1] Super Punch effect
  (if (and (`|EnumEquality` _attackstats_attacktype "MELEE") (`self.Super Punch Ready`))
    (set `UDPlayerAttack.AttackStats` (make `PlayerAttackStats` _attackstats_attacktype_2 (* _attackstats_damage 2) (+ _attackstats_stuntime 3.0)) AttackActor)))

(event `Set Super Punch Cooldown`
  (params (HitData :type "EnemyHitData Structure"))
  (bind _returnvalue (`Actor.K2_GetActorLocation` HitData_Enemy))
  (bind _attackstats_attacktype (break `PlayerAttackStats` (`UDPlayerAttack.AttackStats` HitData_Attack)))
  ;[1 1 1] Put the super punch on cooldown when it hits an enemy. We trigger the cooldown this way so that the super punch isn't expended by meleeing a health pickup.
  (if (and (`|EnumEquality` _attackstats_attacktype "MELEE") (`self.Super Punch Ready`) (not (`|EnumEquality` HitData_EnemyTier "SQUIRE")))
    (bind _output_get (set `self.Upgrade Cooldown Tracker` (`self.Upgrade Cooldown`)))
    (`UDPlayerStatusIcon.StartStatusBar` (`self.Status Widget`) _output_get)
    ;[1 1 1] Punch Explosion
    (`GameplayStatics.PlaySound2D` (`self.Explosion Sound`) 1.0 1.0 0.0 null null)
    (bind _outhit (`KismetSystemLibrary.LineTraceSingleForObjects` (`Actor.K2_GetActorLocation` HitData_Enemy) (* (`Actor.GetActorUpVector` HitData_Enemy) -1000.0) (`|MakeArray` "ObjectTypeQuery1" "ObjectTypeQuery2" "ObjectTypeQuery12" :!type "EObjectTypeQuery Enum"))) ; Find the floor so the particle effect can be spawned there
    (bind _returnvalue_2 (`NiagaraFunctionLibrary.SpawnSystemAtLocation` "/Game/Ursadeath/Upgrades/Blueprints/SuperPunch/NS_SuperPunch.NS_SuperPunch" (`.Location` (`GameplayStatics.BreakHitResult` _outhit))))
    (`NiagaraComponent.SetVariableFloat` _returnvalue_2 "User.Radius" (`self.Blast Radius`))
    (`NiagaraComponent.SetVariableFloat` _returnvalue_2 "User.Effect Height" 10000.0)
    (bind _outhits (`KismetSystemLibrary.SphereTraceMultiForObjects` _returnvalue _returnvalue (`self.Blast Radius`) (`|MakeArray` "ObjectTypeQuery10" :!type "EObjectTypeQuery Enum")))
    (for _array_element _outhits
      (bind _asudenemy (cast `UDEnemy` (`.HitActor` (`GameplayStatics.BreakHitResult` _array_element))))
      (`UDPlayerAttack.ApplyAttackExclusive` HitData_Attack _asudenemy (`UDPlayerAttack.AttackStats` HitData_Attack) 0.0))))

(event `self.TickUpgrade`
  (params (DeltaTime :type "Float (single-precision)"))
  ;[1 1 1] Decrement the upgrade's cooldown.
  (if (not (`self.Super Punch Ready`))
    (set `self.Upgrade Cooldown Tracker` (- (`self.Upgrade Cooldown Tracker`) DeltaTime))
    (`UDPlayerStatusIcon.AddStatusValue` (`self.Status Widget`) (* DeltaTime -1))
    (if (`self.Super Punch Ready`)
      (`GameplayStatics.PlaySound2D` (`self.Recharge Sound`) 1.0 1.0 0.0 null null))))

(fn `Super Punch Ready`
  (returns (`Super Punch Ready` :type Boolean))
  (return (<= (`self.Upgrade Cooldown Tracker`) 0.0)))