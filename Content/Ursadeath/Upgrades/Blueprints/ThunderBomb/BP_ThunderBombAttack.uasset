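; BP_ThunderBombAttack is the attack actor for the Thunder Bomb upgrade, striking all enemies within its explosion radius.
; When the attack finalizes, it spawns a tall Niagara outline at the owning player, scaled to that radius.
; A sphere overlap around the actor finds UDEnemy targets, each receiving a thunder strike effect and exclusive ROCKET-type damage.
; DestroyActor sits inside the enemy loop, so it only runs when a target is hit.
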(event `self.RecieveFinalizeAttack`
  (bind (_attackstats_attacktype _attackstats_damage _attackstats_stuntime) (break `PlayerAttackStats` (`self.AttackStats`)))
  (set `self.AttackStats` (make `PlayerAttackStats` "ROCKET" _attackstats_damage _attackstats_stuntime))
  (bind _returnvalue (`NiagaraFunctionLibrary.SpawnSystemAtLocation` "/Game/Ursadeath/Upgrades/Blueprints/ThunderBomb/NS_ThunderOutline.NS_ThunderOutline" (`self.K2_GetActorLocation` (`self.GetOwningPlayer`))))
  (`NiagaraComponent.SetVariableFloat` _returnvalue "User.Radius" (`self.Explosion Radius`))
  (`NiagaraComponent.SetVariableFloat` _returnvalue "User.Effect Height" 10000.0)
  (bind _outactors (`KismetSystemLibrary.SphereOverlapActors` (`self.K2_GetActorLocation`) (`self.Explosion Radius`) (`|MakeArray` "ObjectTypeQuery10" :!type "EObjectTypeQuery Enum") "/Script/Ursadeath.UDEnemy"))
  (for _array_element _outactors
    (bind _asudenemy (cast `UDEnemy` _array_element))
    (`NiagaraFunctionLibrary.SpawnSystemAtLocation` "/Game/Ursadeath/Upgrades/Blueprints/ThunderBomb/NS_ThunderStrike.NS_ThunderStrike" (`self.K2_GetActorLocation` _asudenemy))
    (`self.ApplyAttackExclusive` _asudenemy (`self.AttackStats`))
    (`self.K2_DestroyActor`)))

(fn `UserConstructionScript`)