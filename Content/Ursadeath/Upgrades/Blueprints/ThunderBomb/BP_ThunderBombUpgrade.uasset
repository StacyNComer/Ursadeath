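; Player upgrade that adds a thunder bomb attack to rocket attacks.
; When added, it binds to the player's attack-spawned event and spawns a thunder attack at the player's location whenever a rocket attack spawns.
; It also attaches a Niagara preview to the player's feet, with its radius taken from the thunder attack's class defaults.
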(event `self.OnUpgradeAdded`
  (params (Player :type "UDPlayerCharacter Object Reference"))
  (add `UDPlayerCharacter.OnAttackSpawned` Player (delegate `Spawn Thunder Attack`))
  (bind _asbp_ursadeath_player (cast `/Game/Ursadeath/PlayerCharacter/Blueprints/BP_UrsadeathPlayer` Player))
  (bind _returnvalue (`NiagaraFunctionLibrary.SpawnSystemAttached` "/Game/Ursadeath/Upgrades/Blueprints/ThunderBomb/NS_ThunderPreview.NS_ThunderPreview" (`/Game/Ursadeath/PlayerCharacter/Blueprints/BP_UrsadeathPlayer.FeetSpawn` _asbp_ursadeath_player) "None" (0.0 0.0 0.0) (struct) "KeepRelativeOffset"))
  (bind _asbp_thunder_bomb_attack (castclass `/Game/Ursadeath/Upgrades/Blueprints/ThunderBomb/BP_ThunderBombAttack` (`self.Attack Class`)))
  (`FXSystemComponent.SetFloatParameter` _returnvalue "User.Radius" (defaults `Object` _asbp_thunder_bomb_attack)))

(event `Spawn Thunder Attack`
  (params (AttackActor :type "UDPlayerAttack Object Reference"))
  (bind _attackstats_attacktype (break `PlayerAttackStats` (`UDPlayerAttack.AttackStats` AttackActor)))
  (bind _owningplayer (`self.OwningPlayer`))
  (if (`|EnumEquality` _attackstats_attacktype "ROCKET")
    (`UDPlayerCharacter.SpawnAttack` :`self` _owningplayer :`AttackClass` (`self.Attack Class`) :`Location` (`Actor.K2_GetActorLocation` _owningplayer))))